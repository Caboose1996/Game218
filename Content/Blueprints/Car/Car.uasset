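; Car interaction actor that lets the player get in and out of a referenced Vehicle when overlapping it.
; Overlap toggles input and shows a prompt; the ActivateThings press is refused if the car is locked (playing a Matinee) or a weapon is ready.
; A FlipFlop alternates entering, which hides and attaches the Character and possesses the Vehicle, with exiting through a DoOnce, which restores the Character and Health widget.
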(event Collision|EventActorBeginOverlap
  (params (OtherActor :type Actor%20Object%20Reference))
  (if (== OtherActor (Game|GetPlayerCharacter 0))
    (Variables|Default|SetSuccess true)
    (Input|EnableInput self (Game|GetPlayerController 0))
    (Development|PrintText "Press \"E\" To Enter Vehicle" true false "(R=0.911000,G=0.969509,B=1.000000,A=1.000000)" 1.0)))

(event Collision|EventActorEndOverlap
  (params (OtherActor :type Actor%20Object%20Reference))
  (if (== OtherActor (Game|GetPlayerCharacter 0))
    (Variables|Default|SetSuccess false)
    (Input|DisableInput self (Game|GetPlayerController 0))))

(event Input|ActionEvents|InputActionActivateThings
  (params (Key :type Key%20Structure :default "AnyKey"))
  (bind _character (Variables|Default|GetCharacter))
  (:Pressed
    (if (Variables|Default|GetIsLocked)
      (Development|PrintString "The Car is Locked")
      (Development|PrintString "Find the Keys")
      (Audio|Components|Audio|Play (Variables|Default|GetMatinee))
      (elif (Variables|/Game/Blueprints/Character/ThirdPersonCharacter.ThirdPersonCharacter_C|GetIsWeaponReady? (Variables|Default|GetCharacter))
        (Development|PrintString "Lower Your Weapons Before Entering Vehicle")
        (else
          (Utilities|FlowControl|FlipFlop
            (:A
              (Variables|/Game/Blueprints/Car/VehicleBlueprint.VehicleBlueprint_C|SetIsInCar? (Variables|Default|GetVehicle) true)
              (Rendering|SetActorHiddenInGame (Pawn|GetControlledPawn (Game|GetPlayerController 0)) true)
              (Rendering|SetActorHiddenInGame (Variables|/Game/Blueprints/Character/ThirdPersonCharacter.ThirdPersonCharacter_C|GetPrimaryRightHandItem (Variables|Default|GetCharacter)) true)
              (Pawn|Possess (Game|GetPlayerController 0) (Variables|Default|GetVehicle)) ; Take control of the pawn
              (Variables|/Game/Blueprints/Car/VehicleBlueprint.VehicleBlueprint_C|SetIsCarOn (Variables|Default|GetVehicle) true)
              (Collision|SetCollisionEnabled (Variables|/Script/Engine.Character|GetCapsuleComponent (Variables|Default|GetCharacter)) "NoCollision")
              (Transformation|AttachActorToActor _character (Variables|Default|GetVehicle) "Person" "KeepWorld" "KeepWorld" "KeepWorld" true)
              (Default|UnattachEquipment _character)
              (Input|EnableInput self (Game|GetPlayerController 0))
              (Viewport|RemoveAllWidgets)
              (goto _label Reset))
            (:B
              (Utilities|FlowControl|DoOnce true :!label _label
                (:Completed
                  (Variables|/Game/Blueprints/Car/VehicleBlueprint.VehicleBlueprint_C|SetIsInCar? (Variables|Default|GetVehicle) false)
                  (Transformation|DetachFromActor (Variables|Default|GetCharacter) "KeepWorld" "KeepRelative" "KeepWorld")
                  (bind _returnvalue (UserInterface|CreateWidget "/Game/Blueprints/Character/Health.Health_C" (Game|GetPlayerController 0)))
                  (UserInterface|Viewport|AddtoViewport _returnvalue 0)
                  (Collision|SetCollisionEnabled (Variables|/Script/Engine.Character|GetCapsuleComponent (Variables|Default|GetCharacter)) "QueryOnly")
                  (Pawn|Possess (Game|GetPlayerController 0) (Variables|Default|GetCharacter))
                  (Rendering|SetActorHiddenInGame (Pawn|GetControlledPawn (Game|GetPlayerController 0)) false)
                  (Rendering|SetActorHiddenInGame (Variables|/Game/Blueprints/Character/ThirdPersonCharacter.ThirdPersonCharacter_C|GetPrimaryRightHandItem (Variables|Default|GetCharacter)) false))))))))))

(fn ConstructionScript)
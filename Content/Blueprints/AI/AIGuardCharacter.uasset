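; AI guard character that patrols a list of waypoint actors using its AI controller.
; BeginPlay caches the controller and sets the first destination to the guard's own location, projected onto the navmesh.
; Tick reissues MoveToLocation every frame; a failed or already-at-goal result waits briefly, then advances the waypoint index and projects that waypoint as the new destination.
; The index resets to zero once it passes the list's end.
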(event EventBeginPlay
  (bind _returnvalue (AI|GetAIController self))
  (Variables|Default|SetAIController _returnvalue)
  (Variables|Default|SetTargetDestination (AI|Navigation|ProjectPointtoNavigation (Transformation|GetActorLocation) (Variables|Default|GetNavData) 0 "0, 0, 0")))

(event Collision|EventActorBeginOverlap
  (params (OtherActor :type Actor%20Object%20Reference)))

(event EventTick
  (params (DeltaSeconds :type Float%20%28single-precision%29))
  (bind _waypoints (Variables|Default|GetWaypoints))
  (bind _returnvalue (AI|Navigation|MovetoLocation (Variables|Default|GetAIController) (Variables|Default|GetTargetDestination) -1.0 true true false))
  (switch Utilities|FlowControl|Switch|SwitchonEPathFollowingRequestResult _returnvalue
    (:Failed
      _)
    (:AlreadyAtGoal
      _))
  (Utilities|FlowControl|Delay 0.2)
  (bind _result (Math|Integer|IncrementInt (Variables|Default|GetCurrentWaypoint))
    (:%20%20
      (if (<= (Variables|Default|GetCurrentWaypoint) (Utilities|Array|Length _waypoints))
        (Variables|Default|SetTargetDestination (AI|Navigation|ProjectPointtoNavigation (Transformation|GetActorLocation (Utilities|Array|Get(acopy) _waypoints _result)) (Variables|Default|GetNavData) 0 "0, 0, 0"))
        (else
          (Variables|Default|SetCurrentWaypoint 0))))))

(fn ConstructionScript)
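; Armed enemy AI character that wanders, investigates noises, shoots at the player on sight and dies when its health runs out.
; Tick repeatedly issues MoveTo toward TargetDestination, picking a random reachable point after a delay when the move fails or arrives.
; PawnSensing retargets that destination and walk speed; sightings also trigger a forward line-trace shot with explosion effect and damage.
; The construction script attaches the gun to the hand socket.
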(event OnSeePawn(PawnSensing)
  (params (Pawn :type Pawn%20Object%20Reference))
  (if (Variables|Default|GetIsAiAlive)
    (Animation|PlayAnimMontage "/Game/AnimStarterPack/RifleIronSights.RifleIronSights" 0.0 "None")
    ;[1 1 1] Sees the Player and moves toward them
    (if (Variables|/Game/Blueprints/Character/ThirdPersonCharacter.ThirdPersonCharacter_C|GetIsPlayerAlive (Variables|Default|GetThirdPerson))
      (Variables|/Script/Engine.CharacterMovementComponent|SetMaxWalkSpeed (Variables|Character|GetCharacterMovement) 6e+02)
      (Variables|Default|SetTargetDestination (AI|Navigation|ProjectPointtoNavigation (Transformation|GetActorLocation Pawn) (Variables|Default|GetNavData) 0 "0, 0, 0"))
      (CallFunction|AIShoot)
      (else
        ;[1 1 1] Moves to Random Locations
        (bind _returnvalue (AI|Navigation|MovetoLocation (Variables|Default|GetAIController) (Variables|Default|GetTargetDestination) -1.0 true true false))
        (switch Utilities|FlowControl|Switch|SwitchonEPathFollowingRequestResult _returnvalue
          (:Failed
            _)
          (:AlreadyAtGoal
            _))
        (Utilities|FlowControl|Delay 3.0)
        (Utilities|FlowControl|DoOnce false :!label _label
          (:Completed
            (Variables|/Script/Engine.CharacterMovementComponent|SetMaxWalkSpeed (Variables|Character|GetCharacterMovement) 2.5e+02)
            (Variables|Default|SetTargetDestination (AI|Navigation|GetRandomReachablePointinRadius (Variables|Default|GetTargetDestination) (Variables|Default|GetWonderRadius) (Variables|Default|GetNavData)))
            (goto _label Reset)))))
    (else
      (Components|Movement|StopMovementImmediately (Variables|Character|GetCharacterMovement)))))

(event OnHearNoise(PawnSensing)
  (params (Instigator :type Pawn%20Object%20Reference) (Location :type Vector%20%28by%20ref%29 :default "0, 0, 0") (Volume :type Float%20%28single-precision%29))
  ;[1 1 1] Hears the Player
  (if (>= Volume (Variables|Default|GetHearingCutoff))
    (Variables|/Script/Engine.CharacterMovementComponent|SetMaxWalkSpeed (Variables|Character|GetCharacterMovement) 1e+02)
    (Variables|Default|SetTargetDestination (AI|Navigation|ProjectPointtoNavigation (Transformation|GetActorLocation Instigator) (Variables|Default|GetNavData) 0 "0, 0, 0"))))

(event Custom|AIShoot
  (bind _staticmesh (Variables|Default|GetStaticMesh))
  (bind _returnvalue (Components|GetOwner _staticmesh))
  (bind _returnvalue_2 (Transformation|GetActorLocation _returnvalue))
  (bind (_x _y _z) (Math|Vector|BreakVector _returnvalue_2))
  (bind _returnvalue_3 (+ _y -2e+01))
  (bind _returnvalue_4 (+ _z 1e+01))
  (bind _returnvalue_5 (Math|Vector|MakeVector _x _returnvalue_3 _returnvalue_4))
  (bind _outhit (Collision|LineTraceByChannel _returnvalue_5 (+ _returnvalue_5 (* (Math|Rotator|GetRotationXVector (Transformation|GetActorRotation (Components|GetOwner _staticmesh))) 2e+03)) "TraceTypeQuery1" false 0 "ForDuration" true "(R=0.445000,G=0.184582,B=0.000000,A=1.000000)" "(R=0.000000,G=1.000000,B=0.000000,A=1.000000)" 0.05))
  (Effects|SpawnEmitteratLocation "/Game/StarterContent/Particles/P_Explosion.P_Explosion" (.Location (Collision|BreakHitResult _outhit)) "0, 0, 0" false)
  (Game|Damage|ApplyDamage (.HitActor (Collision|BreakHitResult _outhit)) 1e+01 0 (Variables|Default|GetAIController)))

(event EventBeginPlay
  ;[1 1 1] Sets up the AI Controller
  (Animation|PlayAnimMontage "/Game/AnimStarterPack/RIfleHip.RIfleHip" 0.0 "None")
  (bind _returnvalue (AI|GetAIController self))
  (Variables|Default|SetAIController _returnvalue)
  (Variables|Default|SetTargetDestination (Transformation|GetActorLocation)))

(event Collision|EventActorBeginOverlap
  (params (OtherActor :type Actor%20Object%20Reference)))

(event EventTick
  (params (DeltaSeconds :type Float%20%28single-precision%29))
  ;[1 1 1] Moves to Random Locations
  (if (Variables|Default|GetIsAiAlive)
    (bind _returnvalue (AI|Navigation|MovetoLocation (Variables|Default|GetAIController) (Variables|Default|GetTargetDestination) -1.0 true true false))
    (switch Utilities|FlowControl|Switch|SwitchonEPathFollowingRequestResult _returnvalue
      (:Failed
        _)
      (:AlreadyAtGoal
        _))
    (Utilities|FlowControl|Delay 3.0)
    (Utilities|FlowControl|DoOnce false :!label _label
      (:Completed
        (Variables|/Script/Engine.CharacterMovementComponent|SetMaxWalkSpeed (Variables|Character|GetCharacterMovement) 2.5e+02)
        (Variables|Default|SetTargetDestination (AI|Navigation|GetRandomReachablePointinRadius (Variables|Default|GetTargetDestination) (Variables|Default|GetWonderRadius) (Variables|Default|GetNavData)))
        (goto _label Reset)))
    (else
      (Components|Movement|StopMovementImmediately (Variables|Character|GetCharacterMovement)))))

(event Game|Damage|EventAnyDamage
  (params (Damage :type Float%20%28single-precision%29) (DamageType :type Damage%20Type%20Object%20Reference) (InstigatedBy :type Controller%20Object%20Reference) (DamageCauser :type Actor%20Object%20Reference))
  (bind _output_get (Variables|Default|SetAI%20Health (- (Variables|Default|GetAI%20Health) (Math|Float|Truncate Damage))))
  (if (<= _output_get 0)
    (Collision|SetCollisionEnabled (Variables|Collision|GetCapsuleComponent) "NoCollision")
    (Collision|SetCollisionEnabled (Variables|Character|GetMesh) "NoCollision")
    (Variables|Default|SetIsAiAlive false)
    (Components|Animation|PlayAnimation (Variables|Character|GetMesh) "/Game/AnimStarterPack/Death_3.Death_3" false)
    (Utilities|FlowControl|Delay 3.0)
    (Actor|DestroyActor)))

(fn ConstructionScript
  (Transformation|AttachComponentToComponent (Variables|Default|GetGun) (Variables|Character|GetMesh) "PrimaryRightHand" "SnapToTarget" "SnapToTarget" "SnapToTarget" true))
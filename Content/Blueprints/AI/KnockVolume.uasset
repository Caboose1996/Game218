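; KnockVolume is a trigger actor that lets the player knock to draw AI characters to their position.
; It enables its own input only while the player pawn overlaps it, disabling it on BeginPlay and on exit.
; Pressing G inside sets every AICharacter's TargetDestination to the player's location projected onto the navmesh.
; Any actor entering also prints a "Knock" message, regardless of whether G is pressed.
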(event EventBeginPlay
  (Input|DisableInput (Game|GetPlayerController 0)))

(event Collision|EventActorBeginOverlap
  (params (OtherActor :type Actor%20Object%20Reference))
  (Development|PrintString "Knock")
  (if (== OtherActor (Game|Player|GetPlayerPawn 0))
    (Input|EnableInput (Game|GetPlayerController 0))))

(event Collision|EventActorEndOverlap
  (params (OtherActor :type Actor%20Object%20Reference))
  (if (== OtherActor (Game|Player|GetPlayerPawn 0))
    (Input|DisableInput (Game|GetPlayerController 0))))

(event Input|KeyboardEvents|G
  (params (Key :type Key%20Structure :default "AnyKey"))
  (:Pressed
    (bind _outactors (Actor|GetAllActorsOfClass "/Game/Blueprints/AI/AICharacter.AICharacter_C"))
    (for _array_element _outactors
      (Variables|/Game/Blueprints/AI/AICharacter.AICharacter_C|SetTargetDestination _array_element (AI|Navigation|ProjectPointtoNavigation (Transformation|GetActorLocation (Game|Player|GetPlayerPawn 0)) (Variables|Default|GetNavData) 0 "0, 0, 0")))))

(fn ConstructionScript)
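; Door actor that opens on a key press while something overlaps it and closes when the overlap ends.
; Actor overlap toggles player 0's input on the door and prints a prompt on entry.
; ActivateThings plays DoorOpen and sets IsDoorOpen, which is never reset.
; Leaving CollisionComponent reverses DoorOpen, with the flag gating only the closing message.
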(event OnComponentEndOverlap(CollisionComponent)
  (params (OverlappedComponent :type Primitive%20Component%20Object%20Reference) (OtherActor :type Actor%20Object%20Reference) (OtherComp :type Primitive%20Component%20Object%20Reference) (OtherBodyIndex :type Integer))
  (Utilities|String|Reverse (Variables|Default|GetDoorOpen))
  (if (Variables|Default|GetIsDoorOpen?)
    (Development|PrintString "Door Closing")))

(event EventBeginPlay)

(event Collision|EventActorBeginOverlap
  (params (OtherActor :type Actor%20Object%20Reference))
  (Input|EnableInput self (Game|GetPlayerController 0))
  (Development|PrintString "Press \"E\" to Open"))

(event EventTick
  (params (DeltaSeconds :type Float%20%28single-precision%29)))

(event Collision|EventActorEndOverlap
  (params (OtherActor :type Actor%20Object%20Reference))
  (Input|DisableInput self (Game|GetPlayerController 0)))

(event Input|ActionEvents|InputActionActivateThings
  (params (Key :type Key%20Structure :default "AnyKey"))
  (:Pressed
    (Audio|Components|Audio|Play (Variables|Default|GetDoorOpen))
    (Variables|Default|SetIsDoorOpen? true)
    (Development|PrintString "Door Open")))

(fn ConstructionScript)
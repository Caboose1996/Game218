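; Power switch actor that lets the player turn on power to ramp controls while standing in its overlap area.
; Overlap enables input and swaps a text render prompt; leaving disables input and restores the exit text.
; Releasing ActivateThings shows the unlocked text, plays the Lights timeline or animation and a sound, and sets IsPowerOn on the referenced RampControls.
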(event EventBeginPlay
  (Rendering|Components|TextRender|SetText (Variables|/Script/Engine.TextRenderActor|GetTextRender (Variables|Default|GetTextRenderActor)) (Utilities|Text|ToText(String) (Variables|Default|GetExit%20Text))))

(event Collision|EventActorBeginOverlap
  (params (OtherActor :type Actor%20Object%20Reference))
  (Rendering|Components|TextRender|SetText (Variables|/Script/Engine.TextRenderActor|GetTextRender (Variables|Default|GetTextRenderActor)) (Utilities|Text|ToText(String) (Variables|Default|GetText)))
  (Input|EnableInput self (Game|GetPlayerController 0)))

(event EventTick
  (params (DeltaSeconds :type Float%20%28single-precision%29)))

(event Collision|EventActorEndOverlap
  (params (OtherActor :type Actor%20Object%20Reference))
  (Rendering|Components|TextRender|SetText (Variables|/Script/Engine.TextRenderActor|GetTextRender (Variables|Default|GetTextRenderActor)) (Utilities|Text|ToText(String) (Variables|Default|GetExit%20Text)))
  (Input|DisableInput self (Game|GetPlayerController 0)))

(event Input|ActionEvents|InputActionActivateThings
  (params (Key :type Key%20Structure :default "AnyKey"))
  (:Released
    (Rendering|Components|TextRender|SetText (Variables|/Script/Engine.TextRenderActor|GetTextRender (Variables|Default|GetTextRenderActor)) (Utilities|Text|ToText(String) (Variables|Default|GetUnlocked)))
    (Audio|Components|Audio|Play (Variables|Default|GetLights))
    (Audio|PlaySoundatLocation (Variables|Default|GetSound) (Transformation|GetActorLocation (Variables|Default|GetPower)))
    (Variables|/Game/Blueprints/Doors/Ramp_Down.Ramp_Down_C|SetIsPowerOn (Variables|Default|GetRampControls) true)))

(fn ConstructionScript)
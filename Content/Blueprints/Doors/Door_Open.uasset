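; A door actor the player opens with the ActivateThings input while standing in its overlap area.
; On player overlap it enables input and prints an "E" prompt; on exit it disables input and reverses the door.
; Pressing the input plays the DoorOpen timeline and sets IsDoorOpen, though the graph here never reads that flag.
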(event EventBeginPlay)

(event Collision|EventActorBeginOverlap
  (params (OtherActor :type Actor%20Object%20Reference))
  (if (== OtherActor (Game|GetPlayerCharacter 0))
    (Variables|Default|SetSuccess? true)
    (Input|EnableInput (Game|GetPlayerController 0))
    (Development|PrintString "Press \"E\" to Open")))

(event EventTick
  (params (DeltaSeconds :type Float%20%28single-precision%29)))

(event Collision|EventActorEndOverlap
  (params (OtherActor :type Actor%20Object%20Reference))
  (if (== OtherActor (Game|GetPlayerCharacter 0))
    (Input|DisableInput self (Game|GetPlayerController 0))
    (Utilities|String|Reverse (Variables|Default|GetDoorOpen))))

(event Input|ActionEvents|InputActionActivateThings
  (params (Key :type Key%20Structure :default "AnyKey"))
  (:Pressed
    (Audio|Components|Audio|Play (Variables|Default|GetDoorOpen))
    (Variables|Default|SetIsDoorOpen? true)))

(fn ConstructionScript)
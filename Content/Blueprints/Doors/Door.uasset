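; Interactive door Blueprint that the player opens with the ActivateThings input while in range.
; A Box overlap enables input from player controller 0 and end overlap disables it, with no check on which actor overlaps.
; Pressing the input prints a debug message and plays Door forward.
; A separate actor-level end overlap event plays Door in reverse.
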(event OnComponentBeginOverlap(Box)
  (params (OverlappedComponent :type Primitive%20Component%20Object%20Reference) (OtherActor :type Actor%20Object%20Reference) (OtherComp :type Primitive%20Component%20Object%20Reference) (OtherBodyIndex :type Integer) (bFromSweep :type Boolean) (SweepResult :type Hit%20Result%20Structure%20%28by%20ref%29))
  (Input|EnableInput self (Game|GetPlayerController 0)))

(event OnComponentEndOverlap(Box)
  (params (OverlappedComponent :type Primitive%20Component%20Object%20Reference) (OtherActor :type Actor%20Object%20Reference) (OtherComp :type Primitive%20Component%20Object%20Reference) (OtherBodyIndex :type Integer))
  (Input|DisableInput self (Game|GetPlayerController 0)))

(event EventBeginPlay)

(event EventTick
  (params (DeltaSeconds :type Float%20%28single-precision%29)))

(event Collision|EventActorEndOverlap
  (params (OtherActor :type Actor%20Object%20Reference))
  (Utilities|String|Reverse (Variables|Default|GetDoor)))

(event Input|ActionEvents|InputActionActivateThings
  (params (Key :type Key%20Structure :default "AnyKey"))
  (:Pressed
    (Development|PrintString "Door Open" true true "(R=0.000000,G=0.660000,B=1.000000,A=1.000000)" 0.5)
    (Audio|Components|Audio|Play (Variables|Default|GetDoor))))

(fn ConstructionScript)
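; Trigger volume for a target-dummy zone that switches the score HUD and eleven dummies on entry and exit.
; Any actor overlap adds a ScoreCounter widget and sets InZone on each individually referenced Dummy.
; End overlap clears InZone, removes all widgets and recreates the Health widget.
; If the player's ThirdPersonCharacter has its weapon ready, exit also restores the Crosshair and resets TimesHit.
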(event EventBeginPlay)

(event Collision|EventActorBeginOverlap
  (params (OtherActor :type Actor%20Object%20Reference))
  (bind _returnvalue (UserInterface|CreateWidget "/Game/Blueprints/Character/ScoreCounter.ScoreCounter_C" (Game|GetPlayerController 0)))
  (UserInterface|Viewport|AddtoViewport _returnvalue 0)
  (Variables|/Game/Blueprints/TargetDummy/TargetDummy.TargetDummy_C|SetInZone? (Variables|Default|GetDummy) true)
  (Variables|/Game/Blueprints/TargetDummy/TargetDummy.TargetDummy_C|SetInZone? (Variables|Default|GetDummy2) true)
  (Variables|/Game/Blueprints/TargetDummy/TargetDummy.TargetDummy_C|SetInZone? (Variables|Default|GetDummy3) true)
  (Variables|/Game/Blueprints/TargetDummy/TargetDummy.TargetDummy_C|SetInZone? (Variables|Default|GetDummy4) true)
  (Variables|/Game/Blueprints/TargetDummy/TargetDummy.TargetDummy_C|SetInZone? (Variables|Default|GetDummy5) true)
  (Variables|/Game/Blueprints/TargetDummy/TargetDummy.TargetDummy_C|SetInZone? (Variables|Default|GetDummy6) true)
  (Variables|/Game/Blueprints/TargetDummy/TargetDummy.TargetDummy_C|SetInZone? (Variables|Default|GetDummy7) true)
  (Variables|/Game/Blueprints/TargetDummy/TargetDummy.TargetDummy_C|SetInZone? (Variables|Default|GetDummy8) true)
  (Variables|/Game/Blueprints/TargetDummy/TargetDummy.TargetDummy_C|SetInZone? (Variables|Default|GetDummy9) true)
  (Variables|/Game/Blueprints/TargetDummy/TargetDummy.TargetDummy_C|SetInZone? (Variables|Default|GetDummy10) true)
  (Variables|/Game/Blueprints/TargetDummy/TargetDummy.TargetDummy_C|SetInZone? (Variables|Default|GetDummy11) true))

(event Collision|EventActorEndOverlap
  (params (OtherActor :type Actor%20Object%20Reference))
  (Variables|/Game/Blueprints/TargetDummy/TargetDummy.TargetDummy_C|SetInZone? (Variables|Default|GetDummy) false)
  (Variables|/Game/Blueprints/TargetDummy/TargetDummy.TargetDummy_C|SetInZone? (Variables|Default|GetDummy2) false)
  (Variables|/Game/Blueprints/TargetDummy/TargetDummy.TargetDummy_C|SetInZone? (Variables|Default|GetDummy3) false)
  (Variables|/Game/Blueprints/TargetDummy/TargetDummy.TargetDummy_C|SetInZone? (Variables|Default|GetDummy4) false)
  (Variables|/Game/Blueprints/TargetDummy/TargetDummy.TargetDummy_C|SetInZone? (Variables|Default|GetDummy5) false)
  (Variables|/Game/Blueprints/TargetDummy/TargetDummy.TargetDummy_C|SetInZone? (Variables|Default|GetDummy6) false)
  (Variables|/Game/Blueprints/TargetDummy/TargetDummy.TargetDummy_C|SetInZone? (Variables|Default|GetDummy7) false)
  (Variables|/Game/Blueprints/TargetDummy/TargetDummy.TargetDummy_C|SetInZone? (Variables|Default|GetDummy8) false)
  (Variables|/Game/Blueprints/TargetDummy/TargetDummy.TargetDummy_C|SetInZone? (Variables|Default|GetDummy9) false)
  (Variables|/Game/Blueprints/TargetDummy/TargetDummy.TargetDummy_C|SetInZone? (Variables|Default|GetDummy10) false)
  (Variables|/Game/Blueprints/TargetDummy/TargetDummy.TargetDummy_C|SetInZone? (Variables|Default|GetDummy11) false)
  (Viewport|RemoveAllWidgets)
  (bind _returnvalue (UserInterface|CreateWidget "/Game/Blueprints/Character/Health.Health_C" (Game|GetPlayerController 0)))
  (UserInterface|Viewport|AddtoViewport _returnvalue 0)
  (bind _asthird_person_character (Utilities|Casting|CastToThirdPersonCharacter (Game|GetPlayerCharacter 0)))
  (if (Variables|/Game/Blueprints/Character/ThirdPersonCharacter.ThirdPersonCharacter_C|GetIsWeaponReady? _asthird_person_character)
    (bind _returnvalue_2 (UserInterface|CreateWidget "/Game/Blueprints/Character/Crosshair.Crosshair_C" (Game|GetPlayerController 0)))
    (UserInterface|Viewport|AddtoViewport _returnvalue_2 0)
    (Variables|/Game/Blueprints/Character/ThirdPersonCharacter.ThirdPersonCharacter_C|SetTimesHit _asthird_person_character 0)))

(event EventTick
  (params (DeltaSeconds :type Float%20%28single-precision%29)))

(fn ConstructionScript)
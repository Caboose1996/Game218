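; Target dummy that reacts to damage while its InZone flag is set, adding to the player character's TimesHit count.
; A hit on a raised dummy swaps between two sets of three point lights and plays a Matinee.
; After timed delays the Matinee reverses and the lights swap back, with IsDummyUp blocking further hits until the reset completes.
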(event EventBeginPlay)

(event Collision|EventActorBeginOverlap
  (params (OtherActor :type Actor%20Object%20Reference)))

(event EventTick
  (params (DeltaSeconds :type Float%20%28single-precision%29)))

(event Game|Damage|EventAnyDamage
  (params (Damage :type Float%20%28single-precision%29) (DamageType :type Damage%20Type%20Object%20Reference) (InstigatedBy :type Controller%20Object%20Reference) (DamageCauser :type Actor%20Object%20Reference))
  (if (Variables|Default|GetInZone?)
    (bind _asthird_person_character (Utilities|Casting|CastToThirdPersonCharacter (Game|GetPlayerCharacter 0)))
    (if (Variables|Default|GetIsDummyUp?)
      (Variables|/Game/Blueprints/Character/ThirdPersonCharacter.ThirdPersonCharacter_C|SetTimesHit _asthird_person_character (+ (Variables|/Game/Blueprints/Character/ThirdPersonCharacter.ThirdPersonCharacter_C|GetTimesHit _asthird_person_character) 1))
      (Rendering|Components|Light|SetIntensity (Variables|Default|GetPointLight1) 0.0)
      (Rendering|Components|Light|SetIntensity (Variables|Default|GetPointLight3) 5e+03)
      (Audio|Components|Audio|Play (Variables|Default|GetMatinee))
      (Variables|Default|SetIsDummyUp? false)
      (Utilities|FlowControl|Delay 3.0)
      (Utilities|String|Reverse (Variables|Default|GetMatinee))
      (Utilities|FlowControl|Delay 2.75)
      (Rendering|Components|Light|SetIntensity (Variables|Default|GetPointLight3) 0.0)
      (Utilities|FlowControl|Delay 0.05)
      (Rendering|Components|Light|SetIntensity (Variables|Default|GetPointLight1) 1e+03)
      (Variables|Default|SetIsDummyUp? true))))

(fn ConstructionScript)
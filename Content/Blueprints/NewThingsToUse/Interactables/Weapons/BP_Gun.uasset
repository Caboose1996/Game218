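; BP_Gun is an interactable hitscan weapon that, on overlap, enables input and sets the player character's ammo and clips.
; Pressing Fire spends a round or triggers the character's reload; if the weapon is ready, it fires and repeats on a timer until release.
; Each shot traces along the owner's instigator aim, spawns an explosion and applies damage.
; Timer shots consume no ammo, and projectile spawning is left unwired.
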(event OnComponentBeginOverlap(InteractableArea)
  (params (OverlappedComponent :type Primitive%20Component%20Object%20Reference) (OtherActor :type Actor%20Object%20Reference) (OtherComp :type Primitive%20Component%20Object%20Reference) (OtherBodyIndex :type Integer) (bFromSweep :type Boolean) (SweepResult :type Hit%20Result%20Structure%20%28by%20ref%29))
  (Input|EnableInput (Game|GetPlayerController 0))
  (bind _asthird_person_character (Utilities|Casting|CastToThirdPersonCharacter (Game|GetPlayerCharacter 0)))
  (Variables|/Game/Blueprints/Character/ThirdPersonCharacter.ThirdPersonCharacter_C|SetClipsSize _asthird_person_character 10)
  (Variables|/Game/Blueprints/Character/ThirdPersonCharacter.ThirdPersonCharacter_C|SetAmmountOfAmmo _asthird_person_character 10)
  (Variables|/Game/Blueprints/Character/ThirdPersonCharacter.ThirdPersonCharacter_C|SetClipsLeft _asthird_person_character 3))

(event Custom|FireWeapon
  (bind _staticmesh (Variables|Default|GetStaticMesh))
  (bind _returnvalue (Transformation|GetWorldLocation _staticmesh))
  (bind (_x _y _z) (Math|Vector|BreakVector _returnvalue))
  (bind _returnvalue_2 (+ _z 0.0))
  (bind _returnvalue_3 (+ _x 0.0))
  (bind _returnvalue_4 (+ _y 0.0))
  (bind _returnvalue_5 (Math|Vector|MakeVector _returnvalue_3 _returnvalue_4 _returnvalue_2))
  (bind _outhit (Collision|LineTraceByChannel _returnvalue_5 (+ _returnvalue_5 (* (Math|Rotator|GetRotationXVector (Pawn|GetBaseAimRotation (Variables|/Script/Engine.Actor|GetInstigator (Components|GetOwner _staticmesh)))) 4e+03)) "TraceTypeQuery2" false (Utilities|Array|MakeArray (Variables|Default|GetThirdPerson)) "None" true "(R=1.000000,G=0.893770,B=0.913795,A=1.000000)" "(R=0.455000,G=0.131135,B=0.000000,A=1.000000)" 5.0))
  (Effects|SpawnEmitteratLocation "/Game/StarterContent/Particles/P_Explosion.P_Explosion" (.Location (Collision|BreakHitResult _outhit)) "0, 0, 0" false)
  (Game|Damage|ApplyDamage (.HitActor (Collision|BreakHitResult _outhit)) 25.0 0 (Variables|Default|GetAIController)))

(event Input|ActionEvents|InputActionFire
  (params (Key :type Key%20Structure :default "AnyKey"))
  (:Pressed
    (bind _asthird_person_character (Utilities|Casting|CastToThirdPersonCharacter (Game|GetPlayerCharacter 0)))
    (if (== (Variables|/Game/Blueprints/Character/ThirdPersonCharacter.ThirdPersonCharacter_C|GetAmmountOfAmmo _asthird_person_character) 0)
      (if (== (Variables|/Game/Blueprints/Character/ThirdPersonCharacter.ThirdPersonCharacter_C|GetClipsLeft _asthird_person_character) 0)
        (Development|PrintString "Out Of Ammo")
        (else
          (Default|Reload _asthird_person_character)
          (Utilities|FlowControl|Delay 0.25)
          (Variables|Default|SetIsReloading true)))
      (elif (Variables|Default|GetIsReloading)
        (Variables|Default|SetIsReloading false)
        (else
          (Variables|/Game/Blueprints/Character/ThirdPersonCharacter.ThirdPersonCharacter_C|SetAmmountOfAmmo _asthird_person_character (- (Variables|/Game/Blueprints/Character/ThirdPersonCharacter.ThirdPersonCharacter_C|GetAmmountOfAmmo _asthird_person_character) 1))
          (if (Variables|/Game/Blueprints/Character/ThirdPersonCharacter.ThirdPersonCharacter_C|GetIsWeaponReady? _asthird_person_character)
            (CallFunction|FireWeapon)
            (Variables|Default|SetIsFiring true)
            (Utilities|Time|SetTimerbyFunctionName 0 "FireWeapon" 0.5 true))))))
  (:Released
    (Variables|Default|SetIsFiring false)
    (Utilities|Time|ClearTimerbyFunctionName 0 "FireWeapon")))

(fn ConstructionScript
  (|CallParentFunction))